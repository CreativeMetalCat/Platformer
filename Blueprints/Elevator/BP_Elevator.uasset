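; BP_Elevator is an elevator actor that moves its static mesh vertically between a start height and an offset Distance.
; Activate starts the movement, and Tick advances it at constant speed, inverting the offset when AtTheEnd is set so each activation reverses direction.
; Start, looping-component and stop sounds accompany the travel, and an OnFinishedMovement dispatcher fires on arrival.
; BeginPlay raises the mesh if AtTheEnd is initially set.
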(event EventBeginPlay
  (bind _startlocation (Variables|Default|GetStartLocation))
  (bind (_x _y _z) (Math|Vector|BreakVector _startlocation))
  (if (Variables|Default|GetAtTheEnd)
    (Transformation|SetWorldLocation (Variables|Default|GetStaticMesh) (Math|Vector|MakeVector _x _y (+ _z (Variables|Movement|GetDistance))) false false)))

(event Collision|EventActorBeginOverlap
  (params (OtherActor :type Actor%20Object%20Reference)))

(event EventTick
  (params (DeltaSeconds :type Float%20%28single-precision%29))
  (bind _distance (Variables|Movement|GetDistance))
  (bind _startlocation (Variables|Default|GetStartLocation))
  (bind (_x _y _z) (Math|Vector|BreakVector _startlocation))
  (if (Variables|Default|GetActivated)
    (Variables|Distance|SetMovedDistance (Math|Interpolation|FInterptoConstant (Variables|Distance|GetMovedDistance) _distance DeltaSeconds (Variables|Movement|GetSpeed)))
    (Transformation|SetWorldLocation (Variables|Default|GetStaticMesh) (Math|Vector|MakeVector _x _y (+ _z (Math|Float|SelectFloat (- _distance (Math|Interpolation|FInterptoConstant (Variables|Distance|GetMovedDistance) _distance DeltaSeconds (Variables|Movement|GetSpeed))) (Math|Interpolation|FInterptoConstant (Variables|Distance|GetMovedDistance) _distance DeltaSeconds (Variables|Movement|GetSpeed)) (Variables|Default|GetAtTheEnd)))) false false)
    (if (>= (Variables|Distance|GetMovedDistance) (Variables|Movement|GetDistance))
      (Audio|PlaySoundatLocation (Variables|Sound|GetStopSound) (Transformation|GetActorLocation) "0, 0, 0" 1.0 1.0 0.0 "/Game/SuperGrid/TutorialLevel/SoundEffects/Attenuation_Ambient.Attenuation_Ambient" 0 0)
      (Audio|Components|Audio|Stop (Variables|Default|GetAudio))
      (Variables|Default|SetActivated false)
      (Variables|Default|SetAtTheEnd (not (Variables|Default|GetAtTheEnd)))
      (Default|CallOnFinishedMovement))))

(fn ConstructionScript
  (Audio|Components|Audio|SetSound (Variables|Default|GetAudio) (Variables|Sound|GetMovementSound))
  (Variables|Default|SetStartLocation (Transformation|GetWorldLocation (Variables|Default|GetStaticMesh))))

(fn Activate
  (Audio|Components|Audio|Play (Variables|Default|GetAudio) 0.0)
  (Variables|Default|SetActivated true)
  (Audio|PlaySoundatLocation (Variables|Sound|GetStartSound) (Transformation|GetActorLocation) "0, 0, 0" 1.0 1.0 0.0 "/Game/SuperGrid/TutorialLevel/SoundEffects/Attenuation_Ambient.Attenuation_Ambient" 0 0)
  (Variables|Distance|SetMovedDistance 0.0))