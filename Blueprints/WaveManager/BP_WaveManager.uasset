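; Wave manager that spawns enemy soldiers from DT_WaveLoadouts rows at placed spawn points and tells the player when a wave ends.
; SpawnNewWaveActors totals a wave's class-to-count map and spawns soldiers, checking spawn-point and max-at-once limits.
; SpawnNewSolder adds single soldiers via ShouldSpawn, cycling spawn points, and overrides a parent class function, as does WaveIdIsValid.
; SpawnNewWave duplicates the spawn logic with separate counters; its completion polling is disconnected.
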(event EventBeginPlay)

(event Collision|EventActorBeginOverlap
  (params (OtherActor :type Actor%20Object%20Reference)))

(event EventTick
  (params (DeltaSeconds :type Float%20%28single-precision%29)))

(event EventSpawnNewWaveActors
  (params (NewWaveId :type Integer))
  (bind _waveloadouts (Variables|Default|GetWaveLoadOuts))
  (Variables|Default|SetAmountOfUsedWaveSpawnPoints 0)
  (if (Utilities|Array|IsValidIndex _waveloadouts NewWaveId)
    (bind _returnvalue (Utilities|GetDataTableRow "/Game/Blueprints/WaveManager/DT_WaveLoadouts.DT_WaveLoadouts" (.RowName (Utilities|Struct|BreakDataTableRowHandle (Utilities|Array|Get(acopy) _waveloadouts NewWaveId))))
      (:then
        (bind _keys (Utilities|Map|Keys (.Enemies (Utilities|Struct|BreakS_WaveLoadout _returnvalue))))
        (bind _values (Utilities|Map|Values (.Enemies (Utilities|Struct|BreakS_WaveLoadout _returnvalue))))
        (for _array_element _values
          (Variables|Default|SetTotalAmountToSpawn (+ (Variables|Default|GetTotalAmountToSpawn) _array_element)))
        (bind (_array_element_2 _array_index) (Utilities|Array|ForEachLoopwithBreak _keys)
          (:LoopBody
            (Utilities|FlowControl|ForLoopwithBreak 0 (- (Utilities|Array|Get(acopy) _values _array_index) 1) :!label _label
              (:LoopBody
                (bind _returnvalue_2 (Game|SpawnActorfromClass _array_element_2 (Transformation|GetActorTransform (Utilities|Array|Get(acopy) (Variables|Default|GetSpawnPoints) (Variables|Default|GetAmountOfUsedWaveSpawnPoints))) "AlwaysSpawn" 0 (Utilities|GetClassDefaults _array_element_2) 0 0 false (Variables|Default|GetWanderingPoints) true 0 0 0 3e+01 "/Game/Customized_Soldier/Materials/Normal/M_Body_6.M_Body_6" "/Game/Customized_Soldier/Materials/Materializing/M_Body_6_Materialize.M_Body_6_Materialize" "/Game/Customized_Soldier/Materials/Materializing/MAT_Heads_Materialize_Inst.MAT_Heads_Materialize_Inst" "/Game/Customized_Soldier/Materials/Normal/MAT_Heads_H_Inst.MAT_Heads_H_Inst" 0.0 0.0 1465.0 true 0 1e+01 1e+01 false false true 0))
                (Utilities|Array|Add (Variables|Default|GetSolders) _returnvalue_2)
                (bind _output_get (Variables|Default|SetAmountOfUsedWaveSpawnPoints (+ (Variables|Default|GetAmountOfUsedWaveSpawnPoints) 1)))
                (bind _result (Math|Integer|IncrementInt (Variables|Default|GetAmountOfSpawned))
                  (:%20%20
                    (if (or (>= _output_get (Utilities|Array|Length (Variables|Default|GetSpawnPoints))) (>= _result (.MaxEnemiesAtOnce (Utilities|Struct|BreakS_WaveLoadout _returnvalue))))
                      (goto _label Break))))))))))))

(event EventProccessEndOfWave
  (Development|PrintString "Wave Completed")
  (Default|DisplayWaveEndMessage (Variables|Default|GetPlayer)))

(fn ConstructionScript)

(fn SpawnNewWave
  (bind _waveloadouts (Variables|Default|GetWaveLoadOuts))
  (if (Utilities|Array|IsValidIndex _waveloadouts (Variables|Default|GetCurrentWaveId))
    (Variables|Default|SetWaveCompleted false)
    (bind _returnvalue (Utilities|GetDataTableRow "/Game/Blueprints/WaveManager/DT_WaveLoadouts.DT_WaveLoadouts" (.RowName (Utilities|Struct|BreakDataTableRowHandle (Utilities|Array|Get(acopy) _waveloadouts (Variables|Default|GetCurrentWaveId)))))
      (:then
        (bind _keys (Utilities|Map|Keys (.Enemies (Utilities|Struct|BreakS_WaveLoadout _returnvalue))))
        (bind _values (Utilities|Map|Values (.Enemies (Utilities|Struct|BreakS_WaveLoadout _returnvalue))))
        (for _array_element _values
          (Variables|Default|SetAmountThatNeedToSpawn (+ (Variables|Default|GetAmountThatNeedToSpawn) _array_element)))
        (bind (_array_element_2 _array_index) (Utilities|Array|ForEachLoopwithBreak _keys)
          (:LoopBody
            (Utilities|FlowControl|ForLoopwithBreak 0 (- (Utilities|Array|Get(acopy) _values _array_index) 1) :!label _label
              (:LoopBody
                (bind _returnvalue_2 (Game|SpawnActorfromClass _array_element_2 (Transformation|GetActorTransform (Utilities|Array|Get(acopy) (Variables|Default|GetSpawnPoints) (LocalVariables|GetWavePointsUsedAmount))) "AlwaysSpawn" 0 (Utilities|GetClassDefaults _array_element_2) 0 0 false (Variables|Default|GetWanderingPoints) true 0 0 0 3e+01 "/Game/Customized_Soldier/Materials/Normal/M_Body_6.M_Body_6" "/Game/Customized_Soldier/Materials/Materializing/M_Body_6_Materialize.M_Body_6_Materialize" "/Game/Customized_Soldier/Materials/Materializing/MAT_Heads_Materialize_Inst.MAT_Heads_Materialize_Inst" "/Game/Customized_Soldier/Materials/Normal/MAT_Heads_H_Inst.MAT_Heads_H_Inst" 0.0 0.0 1465.0 true 0 1e+01 1e+01 false false true 0))
                (Utilities|Array|Add (Variables|Default|GetSpawnedSolders) _returnvalue_2)
                (bind _output_get (LocalVariables|SetWavePointsUsedAmount (+ (LocalVariables|GetWavePointsUsedAmount) 1)))
                (bind _result (Math|Integer|IncrementInt (Variables|Default|GetSpawnedCount))
                  (:%20%20
                    (if (or (>= _output_get (Utilities|Array|Length (Variables|Default|GetSpawnPoints))) (>= _result (.MaxEnemiesAtOnce (Utilities|Struct|BreakS_WaveLoadout _returnvalue))))
                      (goto _label Break)))))))
          (:Completed
            (Variables|Default|SetCurrentWaveId (+ (Variables|Default|GetCurrentWaveId) 1))))))))

(fn GetRandomSpawnPoint
  (params (UsedOnes :type Array%20of%20Integers)))

(fn SpawnNewSolder
  (bind _solders (CallFunction|GetCurrentWaveLoadout))
  (bind _spawnpoints (Variables|Default|GetSpawnPoints))
  (bind _values (Utilities|Map|Values _solders))
  (LocalVariables|SetCount (.TotalCountRes (Class|WaveManagerBase|ShouldSpawn _values (LocalVariables|GetCount))))
  (if (.ReturnValue (Class|WaveManagerBase|ShouldSpawn _values (LocalVariables|GetCount)))
    (bind _keys (Utilities|Map|Keys _solders))
    (if (Utilities|Array|IsValidIndex _spawnpoints (Variables|Default|GetAmountOfUsedWaveSpawnPoints))
      _
      (else
        (Variables|Default|SetAmountOfUsedWaveSpawnPoints 0)))
    (bind _returnvalue (Game|SpawnActorfromClass (Utilities|Array|Get(acopy) _keys (.arrayId (Class|WaveManagerBase|ShouldSpawn _values (LocalVariables|GetCount)))) (Transformation|GetActorTransform (Utilities|Array|Get(acopy) _spawnpoints (Variables|Default|GetAmountOfUsedWaveSpawnPoints))) "AlwaysSpawn" 0 (Utilities|GetClassDefaults (Utilities|Array|Get(acopy) _keys (.arrayId (Class|WaveManagerBase|ShouldSpawn _values (LocalVariables|GetCount))))) 0 0 false 0 true 0 0 0 3e+01 "/Game/Customized_Soldier/Materials/Normal/M_Body_6.M_Body_6" "/Game/Customized_Soldier/Materials/Materializing/M_Body_6_Materialize.M_Body_6_Materialize" "/Game/Customized_Soldier/Materials/Materializing/MAT_Heads_Materialize_Inst.MAT_Heads_Materialize_Inst" "/Game/Customized_Soldier/Materials/Normal/MAT_Heads_H_Inst.MAT_Heads_H_Inst" 0.0 0.0 1465.0 true 0 1e+01 1e+01 false false true 0))
    (Utilities|Array|Add (Variables|Default|GetSolders) 0)
    (return (Utilities|IsValid _returnvalue))
    (else
      (return false))))

(fn GetCurrentWaveLoadout
  (bind _returnvalue (Utilities|GetDataTableRow "/Game/Blueprints/WaveManager/DT_WaveLoadouts.DT_WaveLoadouts" (.RowName (Utilities|Struct|BreakDataTableRowHandle (Utilities|Array|Get(acopy) (Variables|Default|GetWaveLoadOuts) (Variables|Default|GetWaveId)))))
    (:then
      (return (.Enemies (Utilities|Struct|BreakS_WaveLoadout _returnvalue))))))

(fn WaveIdIsValid
  (params (id :type Integer))
  (|CallParentFunction 0)
  (return (Utilities|Array|IsValidIndex (Variables|Default|GetWaveLoadOuts) id)))