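; Per-room wave manager for dungeon mode that locks the player into a fight and marks the room completed afterward.
; Entering the box records the room ID in the game instance, toggles the doors and starts a wave unless already completed or fighting.
; Waves spawn soldiers with tier-based weapons, using difficulty and gamemode data loaded at BeginPlay.
; Wave end toggles the doors again; leaving a completed room clears the player's room state.
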(event OnComponentBeginOverlap(Box)
  (params (OverlappedComponent :type Primitive%20Component%20Object%20Reference) (OtherActor :type Actor%20Object%20Reference) (OtherComp :type Primitive%20Component%20Object%20Reference) (OtherBodyIndex :type Integer) (bFromSweep :type Boolean) (SweepResult :type Hit%20Result%20Structure%20%28by%20ref%29))
  (Utilities|Casting|CastToBP_Player OtherActor)
  (bind _asbp_platformer_game_instance (Utilities|Casting|CastToBP_PlatformerGameInstance (Game|GetGameInstance))
    (:then
      (Variables|/Script/Platformer.PlatformerGameInstance|SetPlayerCurrentRoomId _asbp_platformer_game_instance (Variables|Default|GetRoomId)))
    (:CastFailed
      _))
  (if (and (not (Variables|Default|GetHasBeenCompleted)) (not (Variables|Default|GetIsInFight)))
    (Variables|Default|SetIsInFight true)
    (for _array_element (Variables|Default|GetDoors)
      (Default|Activate _array_element))
    (Class|WaveManagerBase|StartNewWave)
    (bind _asbp_dungeon_player (Utilities|Casting|CastToBP_Dungeon_Player OtherActor))
    (Variables|/Game/Blueprints/Player/BP_Dungeon_Player.BP_Dungeon_Player_C|SetCurrentWaveManager _asbp_dungeon_player self)
    (Default|SetIsinRoom _asbp_dungeon_player true)))

(event OnComponentEndOverlap(Box)
  (params (OverlappedComponent :type Primitive%20Component%20Object%20Reference) (OtherActor :type Actor%20Object%20Reference) (OtherComp :type Primitive%20Component%20Object%20Reference) (OtherBodyIndex :type Integer))
  ;[0.2435 0.5172 1] on leaving the room
  (if (Variables|Default|GetHasBeenCompleted)
    (bind _asbp_dungeon_player (Utilities|Casting|CastToBP_Dungeon_Player OtherActor)
      (:then
        (Default|SetIsinRoom _asbp_dungeon_player false))
      (:CastFailed
        _))
    (bind _asbp_platformer_game_instance (Utilities|Casting|CastToBP_PlatformerGameInstance (Game|GetGameInstance)))
    (if (== (Variables|/Script/Platformer.PlatformerGameInstance|GetPlayerCurrentRoomId _asbp_platformer_game_instance) (Variables|Default|GetRoomId))
      (Variables|/Script/Platformer.PlatformerGameInstance|SetPlayerCurrentRoomId _asbp_platformer_game_instance -1))))

(event EventBeginPlay
  ;[0.6277 1 0.5388] Begin play
  (bind _asbp_platformer_game_instance (Utilities|Casting|CastToBP_PlatformerGameInstance (Game|GetGameInstance)))
  (Variables|Default|SetGamemode (Variables|/Game/Blueprints/Player/BP_PlatformerGameInstance.BP_PlatformerGameInstance_C|GetGamemode _asbp_platformer_game_instance))
  (Variables|Default|SetDifficultyLevel (Variables|/Game/Blueprints/Player/BP_PlatformerGameInstance.BP_PlatformerGameInstance_C|GetDifficulty _asbp_platformer_game_instance))
  (CallFunction|LoadDifficultyandGamemodeData))

(event Collision|EventActorBeginOverlap
  (params (OtherActor :type Actor%20Object%20Reference))
  (|CallParentFunction OtherActor) ; This node is disabled and will not be called.\nDrag off pins to build functionality.
)

(event EventTick
  (params (DeltaSeconds :type Float%20%28single-precision%29))
  (|CallParentFunction DeltaSeconds) ; This node is disabled and will not be called.\nDrag off pins to build functionality.
)

(event EventProccessEndOfWave
  ;[0.3728 1 0.9502] On wave end
  (Default|CallOnWaveCompleted)
  (Development|PrintString "Wave Completed. Now to the next room" true false)
  (Variables|Default|SetHasBeenCompleted true)
  (Variables|Default|SetIsInFight false)
  (for _array_element (Variables|Default|GetDoors)
    (Default|Activate _array_element)))

(event EventSpawnNewWaveActors
  (params (NewWaveId :type Integer))
  (bind _money_enemytospawncount (Variables|Default|GetMoney_EnemyToSpawnCount))
  ;[0.763 0.4463 1] Generate wave
  (bind _weaponclass (CallFunction|GetWeaponBasedonTier))
  (Variables|Default|SetAvailableWeapons _weaponclass)
  (Variables|Default|SetCurrentWaveLoadout (Utilities|Struct|MakeS_WaveLoadout (Utilities|Map|MakeMap "/Game/Blueprints/AI/BP_Solder.BP_Solder_C" _money_enemytospawncount) _money_enemytospawncount))
  (CallFunction|SpawnActorFowLoadOut))

(fn ConstructionScript
  (|CallParentFunction))