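; BP_Teleport is an interactable teleporter that moves whoever uses it to the location of a destination actor.
; On Interact, if usable and the destination is valid, it relocates the interactor without a sweep and calls the OnIntreacted dispatcher.
; It then plays its interaction sound plus a particle burst and electric sound at the arrival point.
; A one-shot timer re-enables the teleporter after a configurable cooldown.
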(event Custom|ReActivate
  (Variables|Default|SetCanBeUsed true))

(event EventBeginPlay
  (|CallParentFunction) ; This node is disabled and will not be called.\nDrag off pins to build functionality.
)

(event Collision|EventActorBeginOverlap
  (params (OtherActor :type Actor%20Object%20Reference))
  (|CallParentFunction OtherActor) ; This node is disabled and will not be called.\nDrag off pins to build functionality.
)

(event EventTick
  (params (DeltaSeconds :type Float%20%28single-precision%29))
  (|CallParentFunction DeltaSeconds) ; This node is disabled and will not be called.\nDrag off pins to build functionality.
)

(event EventInteract
  (params (Interactor :type Actor%20Object%20Reference))
  (bind _returnvalue (Transformation|GetActorLocation Interactor))
  (bind _destinationactor (Variables|Default|GetDestinationActor))
  (if (Variables|Default|GetCanBeUsed)
    (Utilities|IsValid _destinationactor
      (:Is%20Valid
        (Transformation|SetActorLocation Interactor (Transformation|GetActorLocation _destinationactor) false false)
        (Default|CallOnIntreacted self Interactor)
        (Audio|Components|Audio|Play (Variables|Default|GetInteractionSound) 0.0)
        (Effects|SpawnEmitteratLocation "/Game/AdvancedMagicFX12/particles/P_ky_hit_shine.P_ky_hit_shine" _returnvalue)
        (Audio|PlaySoundatLocation "/Game/Sounds/hl2/ambient/levels/labs/electric_explosion5.electric_explosion5" _returnvalue "0, 0, 0" 1.0 1.0 0.0 "/Game/SuperGrid/TutorialLevel/SoundEffects/Attenuation_Ambient.Attenuation_Ambient" 0 0)
        (Utilities|Time|SetTimerbyEvent (delegate Custom|ReActivate) (Variables|Default|GetCooldownTime))
        (Variables|Default|SetCanBeUsed false)))))

(fn ConstructionScript
  (|CallParentFunction))