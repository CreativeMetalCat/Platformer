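; AI controller for soldiers that wander between points and shoot enemies they see.
; Init runs a behavior tree, then either locks onto a pawn-supplied target or starts a looping timer feeding sight perception into UpdateAI to trigger shooting.
; Pawn interface messages supply wander points and toggle aiming on target found or lost, while a timeout timer replaces unreached points.
; Older inline targeting and hearing logic remains disconnected.
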(event Custom|UpdateAIEvent
  (bind _returnvalue (Class|SolderAiBase|UpdateAI (Class|AIPerceptionComponent|GetPerceivedActors (Variables|Default|GetAIPerception) "/Script/AIModule.AISense_Sight")))
  (if _returnvalue
    (Class|IAI|ShootatTarget(Message) (Pawn|GetControlledPawn) (Variables|Default|GetCurrentEnemy))))

(event Custom|Init
  (bind _returnvalue (Pawn|GetControlledPawn))
  (Class|SolderAiBase|ResetGiveUpTimer)
  (AI|RunBehaviorTree (Variables|Default|GetBehaviorTree))
  (bind _can (Class|IAI|GetCanAlwaysSeeTarget(Message) _returnvalue))
  (if (not _can)
    (bind _returnvalue_2 (Utilities|Time|SetTimerbyEvent (delegate Custom|UpdateAIEvent) 0.1 true))
    (Variables|Default|SetAIUpdateTimerHandle _returnvalue_2)
    (bind _point (Class|IAI|GetPointtoWanderto(Message) (Pawn|GetControlledPawn)))
    (AI|Components|Blackboard|SetValueasObject (Variables|Default|GetBlackboard) (Utilities|Name|MakeLiteralName "WanderPoint") _point)
    (else
      (bind _targetactor (Class|IAI|GetTarget(Message) _returnvalue))
      (CallFunction|SetTarget _targetactor))))

(event EventOnEnemyLost
  (Class|IAI|ChangeAiming(Message) (Pawn|GetControlledPawn) false)
  (bind _returnvalue (Utilities|Time|SetTimerbyEvent (delegate EventOnReachedPointOfWander) (Variables|Default|GetMaxTimeToReachPoint)))
  (Variables|Default|SetFailToReachWanderPointTimerHandle _returnvalue))

(event EventTick
  (params (DeltaSeconds :type Float%20%28single-precision%29)))

(event EventOnReachedLastSeenLocation
  (AI|Components|Blackboard|ClearValue (Variables|Default|GetBlackboard) (Utilities|Name|MakeLiteralName "LastSeenLocation")))

(event EventOnReachedPointOfWander
  (bind _point (Class|IAI|GetPointtoWanderto(Message) (Pawn|GetControlledPawn)))
  (AI|Components|Blackboard|SetValueasObject (Variables|Default|GetBlackboard) (Utilities|Name|MakeLiteralName "WanderPoint") _point)
  (bind _returnvalue (Utilities|Time|SetTimerbyEvent (delegate EventOnReachedPointOfWander) (Variables|Default|GetMaxTimeToReachPoint)))
  (Variables|Default|SetFailToReachWanderPointTimerHandle _returnvalue))

(event EventOnTargetFound
  (Class|IAI|ChangeAiming(Message) (Pawn|GetControlledPawn) true))

(event EventSelectNewWanderPoint
  (bind _point (Class|IAI|GetPointtoWanderto(Message) (Pawn|GetControlledPawn)))
  (AI|Components|Blackboard|SetValueasObject (Variables|Default|GetBlackboard) (Utilities|Name|MakeLiteralName "WanderPoint") _point)
  (bind _returnvalue (Utilities|Time|SetTimerbyEvent (delegate EventOnReachedPointOfWander) (Variables|Default|GetMaxTimeToReachPoint)))
  (Variables|Default|SetFailToReachWanderPointTimerHandle _returnvalue))

(fn ConstructionScript)

(fn FindSuitableLastLocation
  (bind _outactors (Actor|GetAllActorsOfClass "/Game/Blueprints/AI/ImportantPointsSystem/BP_ImportantPoint.BP_ImportantPoint_C"))
  (for (_array_element _array_index) _outactors
    (if (or (== (LocalVariables|GetClosestId) -1) (< (Math|Vector|Distance(Vector) (Transformation|GetActorLocation _array_element) (Transformation|GetActorLocation)) (LocalVariables|GetClosest)))
      (LocalVariables|SetClosestId _array_index)
      (LocalVariables|SetClosest (Math|Vector|Distance(Vector) (Transformation|GetActorLocation _array_element) (Transformation|GetActorLocation)))))
  (if (!= (LocalVariables|GetClosestId) -1)
    (return (Transformation|GetActorLocation (Utilities|Array|Get(acopy) _outactors (LocalVariables|GetClosestId))) true)
    (else
      (return "0, 0, 0" false))))

(fn SetTarget
  (params (Target :type Actor%20Object%20Reference))
  (bind _output_get (Variables|Default|SetTarget Target))
  (AI|Components|Blackboard|SetValueasObject (Variables|Default|GetBlackboard) (Utilities|Name|MakeLiteralName "Target") _output_get)
  (AI|SetFocus _output_get))

(fn IsTargetAlive
  (params (Object :type Object%20Object%20Reference))
  (Utilities|IsValid Object
    (:Is%20Valid
      (return (not (Default|GetIsDead (.AsBP%20Human%20Base (Utilities|Casting|CastToBP_HumanBase Object))))))
    (:Is%20Not%20Valid
      (return false))))

(fn GetCanAlwaysSeeTarget
  (return false))

(fn GetCurrentWanderTarget
  (bind _blackboard (Variables|Default|GetBlackboard))
  (Utilities|IsValid _blackboard
    (:Is%20Valid
      (return (.AsActor (Utilities|Casting|CastToActor (AI|Components|Blackboard|GetValueasObject _blackboard (Utilities|Name|MakeLiteralName "WanderPoint"))))))))

(fn GetLastSeenLocation
  (return (Variables|Default|GetLastSeenLocation)))

(fn GetPointtoWanderto
  (return 0))

(fn GetTarget
  (return (Variables|Default|GetCurrentEnemy)))