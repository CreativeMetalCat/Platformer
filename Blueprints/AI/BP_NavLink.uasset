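; Nav link that makes BP_HumanBase agents jump, either on reaching the smart link or on entering a trigger at either end.
; The construction script moves the left and right jump triggers onto the link's points.
; UseSmartLink selects the mode; trigger mode excludes BP_Player.
; ShouldJump compares Y velocity with the target point's direction, but its result is ignored, so smart-link agents always jump.
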(event OnComponentBeginOverlap(TriggerJumpLeft)
  (params (OverlappedComponent :type Primitive%20Component%20Object%20Reference) (OtherActor :type Actor%20Object%20Reference) (OtherComp :type Primitive%20Component%20Object%20Reference) (OtherBodyIndex :type Integer) (bFromSweep :type Boolean) (SweepResult :type Hit%20Result%20Structure%20%28by%20ref%29))
  (CallFunction|Jump OtherActor))

(event OnComponentBeginOverlap(TriggerJumpRight)
  (params (OverlappedComponent :type Primitive%20Component%20Object%20Reference) (OtherActor :type Actor%20Object%20Reference) (OtherComp :type Primitive%20Component%20Object%20Reference) (OtherBodyIndex :type Integer) (bFromSweep :type Boolean) (SweepResult :type Hit%20Result%20Structure%20%28by%20ref%29))
  (CallFunction|Jump OtherActor))

(event EventBeginPlay
  (Collision|SetActorEnableCollision true))

(event Collision|EventActorBeginOverlap
  (params (OtherActor :type Actor%20Object%20Reference)))

(event EventTick
  (params (DeltaSeconds :type Float%20%28single-precision%29)))

(event EventSmartLinkReached
  (params (Agent :type Actor%20Object%20Reference) (Destination :type Vector%20%28by%20ref%29 :default "0, 0, 0"))
  (if (Variables|Default|GetUseSmartLink)
    (if (CallFunction|ShouldJump Agent)
      _
      (else
        _))
    (bind _asbp_human_base (Utilities|Casting|CastToBP_HumanBase Agent))
    (Character|Jump _asbp_human_base)))

(fn ConstructionScript
  (bind (_exists _returnvalue) (Class|NavLinkProxyBlueprintBase|GetLeftPoint))
  (if _exists
    (Transformation|SetRelativeLocation (Variables|Default|GetTriggerJumpLeft) _returnvalue false false)
    (Transformation|SetRelativeLocation (Variables|Default|GetTriggerJumpRight) (.ReturnValue (Class|NavLinkProxyBlueprintBase|GetRightPoint)) false false)))

(fn Jump
  (params (Object :type Actor%20Object%20Reference))
  (if (not (Variables|Default|GetUseSmartLink))
    (bind _asbp_human_base (Utilities|Casting|CastToBP_HumanBase Object))
    (Utilities|Casting|CastToBP_Player _asbp_human_base
      (:CastFailed
        (Character|Jump _asbp_human_base)))))

(fn ShouldJump
  (params (Agent :type Actor%20Object%20Reference))
  (bind _returnvalue (Transformation|GetVelocity))
  (bind _returnvalue_2 (Transformation|GetVelocity Agent))
  (bind _returnvalue_3 (Class|NavLinkProxyBlueprintBase|GetRightPoint))
  (bind _returnvalue_4 (Class|NavLinkProxyBlueprintBase|GetLeftPoint))
  (bind _returnvalue_5 (Transformation|GetActorLocation))
  (bind _returnvalue_6 (Transformation|GetActorLocation))
  (bind _y (Math|Vector|BreakVector _returnvalue_2))
  (bind _y_2 (Math|Vector|BreakVector _returnvalue))
  (bind _returnvalue_7 (+ _returnvalue_4 _returnvalue_5))
  (bind _returnvalue_8 (+ _returnvalue_3 _returnvalue_6))
  (bind _infront (CallFunction|GetPointRelationtoPlayer _returnvalue_8 Agent))
  (bind _infront_2 (CallFunction|GetPointRelationtoPlayer _returnvalue_7 Agent))
  (if (CallFunction|GetIsOverlappingThisThigger (Variables|Default|GetTriggerJumpLeft) Agent)
    (if (and _infront (> _y 0.0))
      _
      (elif (and (not _infront) (< _y 0.0))
        _
        (else
          (return false))))
    (return true)
    (else
      (if (and _infront_2 (> _y_2 0.0))
        _
        (elif (and (not _infront_2) (< _y_2 0.0))
          _
          (else
            (return false))))
      (return true))))

(fn GetIsOverlappingThisThigger
  (params (Collision :type Box%20Component%20Object%20Reference) (Agent :type Actor%20Object%20Reference))
  (for _array_element (Collision|GetOverlappingActors Collision (Utilities|GetClass Agent) :!class /Script/Engine.PrimitiveComponent)
    (if (== _array_element Agent)
      (return true)))
  (return false))

(fn GetPointRelationtoPlayer
  (params (Point :type Vector) (Agent :type Actor%20Object%20Reference))
  (return (> (- (.Y (Math|Vector|BreakVector Point)) (.Y (Math|Vector|BreakVector (Transformation|GetActorLocation Agent)))) 0.0)))