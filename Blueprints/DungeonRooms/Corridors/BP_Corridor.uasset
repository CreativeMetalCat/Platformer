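; BP_Corridor is a dungeon corridor piece that configures its four walls and shows itself only while the player is inside its trigger box.
; GenerateWalls sets wall visibility and query collision from per-side flags.
; For drops, it reveals drop meshes on the relevant ends, and the start-linked case spawns a BP_Teleport targeting the DropStart corridor's result location.
; Box overlaps drive SetEnabled, which hides or shows the actor and its static meshes.
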(event OnComponentBeginOverlap(Box)
  (params (OverlappedComponent :type Primitive%20Component%20Object%20Reference) (OtherActor :type Actor%20Object%20Reference) (OtherComp :type Primitive%20Component%20Object%20Reference) (OtherBodyIndex :type Integer) (bFromSweep :type Boolean) (SweepResult :type Hit%20Result%20Structure%20%28by%20ref%29))
  (Utilities|Casting|CastToBP_Player OtherActor)
  (CallFunction|SetEnabled true))

(event OnComponentEndOverlap(Box)
  (params (OverlappedComponent :type Primitive%20Component%20Object%20Reference) (OtherActor :type Actor%20Object%20Reference) (OtherComp :type Primitive%20Component%20Object%20Reference) (OtherBodyIndex :type Integer))
  (Utilities|Casting|CastToBP_Player OtherActor)
  (CallFunction|SetEnabled false))

(event EventBeginPlay)

(event Collision|EventActorBeginOverlap
  (params (OtherActor :type Actor%20Object%20Reference)))

(event EventTick
  (params (DeltaSeconds :type Float%20%28single-precision%29)))

(event EventGenerateWalls
  (bind _hasupwall (Variables|Default|GetHasUpWall))
  (bind _hasdownwall (Variables|Default|GetHasDownWall))
  (bind _hasrightwall (Variables|Default|GetHasRightWall))
  (bind _downdrop (Variables|Default|GetDownDrop))
  (bind _hasleftwall (Variables|Default|GetHasLeftWall))
  (Rendering|SetVisibility (Variables|Default|GetUp) _hasupwall false)
  (Rendering|SetVisibility (Variables|Default|GetDown) _hasdownwall false)
  (Rendering|SetVisibility (Variables|Default|GetRight) _hasrightwall false)
  (Rendering|SetVisibility (Variables|Default|GetLeft) _hasleftwall false)
  (Collision|SetCollisionEnabled (Variables|Default|GetRight) (select _hasrightwall "QueryOnly" "NoCollision"))
  (Collision|SetCollisionEnabled (Variables|Default|GetLeft) (select _hasleftwall "QueryOnly" "NoCollision"))
  (Collision|SetCollisionEnabled (Variables|Default|GetDown) (select _hasdownwall "QueryOnly" "NoCollision"))
  (Collision|SetCollisionEnabled (Variables|Default|GetUp) (select _hasupwall "QueryOnly" "NoCollision"))
  (if (Variables|Default|GetbIsDrop)
    (if (!= (Variables|Default|GetIdOfDropEnd) -1)
      (Rendering|SetVisibility (Variables|Default|GetDown) false false)
      (Rendering|SetVisibility _downdrop true false)
      (Collision|SetCollisionEnabled _downdrop "QueryOnly"))
    (if (!= (Variables|Default|GetIdOfDropStart) -1)
      (Rendering|SetVisibility (Variables|Default|GetUp) false false)
      (Rendering|SetVisibility (Variables|Default|GetUpDrop1) true false)
      (Collision|SetCollisionEnabled (Variables|Default|GetUpDrop) "QueryOnly")
      (bind _asbp_corridor (Utilities|Casting|CastToBP_Corridor (Variables|Default|GetDropStart)))
      (Game|SpawnActorfromClass "/Game/Blueprints/Movement/BP_Teleport.BP_Teleport_C" (Transformation|GetWorldTransform (Variables|Default|GetTeleportSpawnLocation)) "AlwaysSpawn" 0 0 true 0.01 (Transformation|GetWorldLocation (Variables|BP_Corridor_C|GetTeleportResultLocation _asbp_corridor)) 0))))

(fn ConstructionScript)

(fn SetEnabled
  (params (Is :type Boolean))
  (bind _returnvalue (not Is))
  (Rendering|SetActorHiddenInGame _returnvalue)
  (for _array_element (Actor|GetComponentsByClass "/Script/Engine.StaticMeshComponent")
    (Development|SetHiddeninGame _array_element _returnvalue false))
  (Variables|Default|SetEnabled Is))