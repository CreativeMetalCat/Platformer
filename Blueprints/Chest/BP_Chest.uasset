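; Locked loot chest that a dungeon player opens with a matching key to receive a random pickup.
; Interact consumes the key, plays a sound and a timeline lid rotation, then activates Niagara and spawns ammo, health, armor, money, customization item or weapon from PossibleItems.
; Each type check and value read re-rolls the random index, so they can mix entries.
; Used is set false on opening, so the chest never becomes spent.
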(event EventBeginPlay)

(event Collision|EventActorBeginOverlap
  (params (OtherActor :type Actor%20Object%20Reference)))

(event EventTick
  (params (DeltaSeconds :type Float%20%28single-precision%29)))

(event EventInteract
  (params (Interactor :type Actor%20Object%20Reference))
  (bind _neededkey (Variables|Default|GetNeededKey))
  (bind _possibleitems (Variables|Default|GetPossibleItems))
  (bind _itemspawnpoint (Variables|Default|GetItemSpawnPoint))
  (bind _itemspawnpoint_2 (Variables|Default|GetItemSpawnPoint))
  (bind _returnvalue (Utilities|Array|Length _possibleitems))
  (bind _returnvalue_2 (Transformation|GetWorldTransform _itemspawnpoint))
  (bind _returnvalue_3 (Transformation|GetWorldTransform _itemspawnpoint_2))
  (bind _returnvalue_4 (Math|Random|RandomInteger _returnvalue))
  (bind _output (Utilities|Array|Get(acopy) _possibleitems _returnvalue_4))
  (bind (_canbesoldout _name _description _price _isammo _ammocategory _ammoamount _weaponstatsinfo _weaponclass _image _ishealthkit _healthamount _isarmor _armorhealth _ismoney _moneyamount _iscustomizationitem _customizationitem) (Utilities|Struct|BreakS_StoreItemInfo _output))
  (if (not (Variables|Default|GetUsed))
    (bind _asbp_dungeon_player (Utilities|Casting|CastToBP_Dungeon_Player Interactor))
    (if (Default|HasKey _asbp_dungeon_player _neededkey)
      (Default|UseKey _asbp_dungeon_player _neededkey)
      (Variables|Default|SetUsed false)
      (Audio|Components|Audio|Play (Variables|Default|GetInteractionSound) 0.0)
      (bind _rotation (Timeline|ChestOpenAnim PlayFromStart)
        (:Update
          (Transformation|SetRelativeRotation (Variables|Default|GetSM_Chest_01d) (Math|Rotator|MakeRotator (* _rotation -1.1e+02) 0.0 -9e+01) false false))
        (:Finished
          (Components|Activation|Activate (Variables|Default|GetNiagara) true)
          (if _isammo
            (Game|SpawnActorfromClass "/Game/Blueprints/PickUps/BP_AmmoPickup.BP_AmmoPickup_C" _returnvalue_3 "AlwaysSpawn" 0 (Utilities|Map|MakeMap _ammocategory _ammoamount) true false 15.0 "/Game/Sounds/hl2beta/weapons/misc/ammo_pickup.ammo_pickup" false 0 true 0)
            (elif _ishealthkit
              (Game|SpawnActorfromClass "/Game/Blueprints/PickUps/BP_HealthPickup.BP_HealthPickup_C" _returnvalue_3 "AlwaysSpawn" 0 (Math|Conversions|ToFloat(Integer) _healthamount) false 0.0 "/Game/Sounds/hl2beta/weapons/misc/ammo_pickup.ammo_pickup" false 0 true 0)
              (elif _isarmor
                (Game|SpawnActorfromClass "/Game/Blueprints/PickUps/BP_ArmorPickup.BP_ArmorPickup_C" _returnvalue_2 "AlwaysSpawn" 0 (Math|Conversions|ToFloat(Integer) _armorhealth) false 0.0 "/Game/Sounds/hl2beta/weapons/misc/ammo_pickup.ammo_pickup" false 0 true 0)
                (elif _ismoney
                  (Game|SpawnActorfromClass "/Game/Blueprints/PickUps/BP_MoneyPickup.BP_MoneyPickup_C" _returnvalue_2 "AlwaysSpawn" 0 _moneyamount false 0.0 "/Game/Sounds/hl2beta/weapons/misc/ammo_pickup.ammo_pickup" false 0 true 0)
                  (elif _iscustomizationitem
                    (Game|SpawnActorfromClass "/Game/Blueprints/PickUps/BP_ItemPickup.BP_ItemPickup_C" _returnvalue_2 "AlwaysSpawn" 0 _customizationitem false 0.0 "/Game/Sounds/hl2beta/weapons/misc/ammo_pickup.ammo_pickup" true 0 true 0)
                    (else
                      (Game|SpawnActorfromClass _weaponclass _returnvalue_2 "AlwaysSpawn" 0 (.DefaultAmmoInTheClip (Utilities|GetClassDefaults _weaponclass)) true 0))))))))))))

(fn ConstructionScript)