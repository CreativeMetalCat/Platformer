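; BP_BTR is a configurable BTR armored personnel carrier actor with BTR-70 and BTR-152 variants.
; The construction script uses Type to pick the skeletal mesh, ColorScheme to set its materials, and HasCollision to toggle collision.
; The turretless BTR-70 hides its turret bone in construction and again on BeginPlay, which also hides bones listed in WheelsToHide.
; The BTR-152 without a back wheel uses a separate mesh.
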(event EventBeginPlay
  (if (Utilities|Enum|Equal(Enum) (Variables|Default|GetType) "NewEnumerator3")
    (Components|SkinnedMesh|HideBonebyName (Variables|Default|GetSM_BTR) "Turret" "PBO_Term"))
  (for _array_element (Variables|Default|GetWheelsToHide)
    (Components|SkinnedMesh|HideBonebyName (Variables|Default|GetSM_BTR) (Utilities|String|StringToName _array_element) "PBO_Term")))

(event Collision|EventActorBeginOverlap
  (params (OtherActor :type Actor%20Object%20Reference)))

(event EventTick
  (params (DeltaSeconds :type Float%20%28single-precision%29)))

(fn ConstructionScript
  (bind _sm_btr (Variables|Default|GetSM_BTR))
  (bind _colorscheme (Variables|Default|GetColorScheme))
  (switch Utilities|FlowControl|Switch|SwitchonE_BTRType (Variables|Default|GetType)
    (:NewEnumerator0
      (Class|SkinnedMeshComponent|SetSkeletalMesh _sm_btr "/Game/models/VH_BTR70/Meshes/SM_BTR70.SM_BTR70" true)
      (Rendering|Material|SetMaterial _sm_btr 0 (Utilities|Select :Index _colorscheme :NewEnumerator0 "/Game/models/VH_BTR70/Materials/MI_BTR70_Turret_Beige.MI_BTR70_Turret_Beige" :NewEnumerator1 "/Game/models/VH_BTR70/Materials/MI_BTR70_Turret_Urban_Beige.MI_BTR70_Turret_Urban_Beige" :NewEnumerator2 "/Game/models/VH_BTR70/Materials/MI_BTR70_Turret_Black.MI_BTR70_Turret_Black" :NewEnumerator3 "/Game/models/VH_BTR70/Materials/MI_BTR70_Turret_Forrest_Green.MI_BTR70_Turret_Forrest_Green" :NewEnumerator4 "/Game/models/VH_BTR70/Materials/MI_BTR70_Turret_White.MI_BTR70_Turret_White" :NewEnumerator5 "/Game/models/VH_BTR70/Materials/M_BTR70_Turret_Green.M_BTR70_Turret_Green") :!label _label)
      (Rendering|Material|SetMaterial _sm_btr 2 (Utilities|Select :Index _colorscheme :NewEnumerator0 "/Game/models/VH_BTR70/Materials/MI_BTR70_Body_Beige.MI_BTR70_Body_Beige" :NewEnumerator1 "/Game/models/VH_BTR70/Materials/MI_BTR70_Body_Urban_Beige.MI_BTR70_Body_Urban_Beige" :NewEnumerator2 "/Game/models/VH_BTR70/Materials/MI_BTR70_Body_Black.MI_BTR70_Body_Black" :NewEnumerator3 "/Game/models/VH_BTR70/Materials/MI_BTR70_Body_Forrest_Green.MI_BTR70_Body_Forrest_Green" :NewEnumerator4 "/Game/models/VH_BTR70/Materials/MI_BTR70_Body_White.MI_BTR70_Body_White" :NewEnumerator5 "/Game/models/VH_BTR70/Materials/M_BTR70_Body_Green.M_BTR70_Body_Green")))
    (:NewEnumerator3
      (Class|SkinnedMeshComponent|SetSkeletalMesh _sm_btr "/Game/models/VH_BTR70/Meshes/SM_BTR70.SM_BTR70" true)
      (Components|SkinnedMesh|HideBonebyName (Variables|Default|GetSM_BTR) "Turret" "PBO_Term")
      (goto _label))
    (:NewEnumerator1
      (Class|SkinnedMeshComponent|SetSkeletalMesh _sm_btr "/Game/models/VH_BTR152/Meshes/SK_BTR152.SK_BTR152" true)
      (Rendering|Material|SetMaterial (Variables|Default|GetSM_BTR) 1 (Utilities|Select :Index _colorscheme :NewEnumerator0 "/Game/models/VH_BTR152/Materials/MI_BTR152_Beige.MI_BTR152_Beige" :NewEnumerator1 "/Game/models/VH_BTR152/Materials/MI_BTR152_Beige_Urban.MI_BTR152_Beige_Urban" :NewEnumerator2 "/Game/models/VH_BTR152/Materials/MI_BTR152_Blue.MI_BTR152_Blue" :NewEnumerator3 "/Game/models/VH_BTR152/Materials/MI_BTR152_Green_Forest.MI_BTR152_Green_Forest" :NewEnumerator4 "/Game/models/VH_BTR152/Materials/MI_BTR152_White.MI_BTR152_White" :NewEnumerator5 "/Game/models/VH_BTR152/Materials/M_BTR152_Green.M_BTR152_Green") :!label _label_2))
    (:NewEnumerator2
      (Class|SkinnedMeshComponent|SetSkeletalMesh _sm_btr "/Game/models/VH_BTR152/Meshes/NoBackWheel/SK_BTR152_NoBackWheel.SK_BTR152_NoBackWheel" true)
      (goto _label_2)))
  (Collision|SetCollisionEnabled (Variables|Default|GetSM_BTR) (select (Variables|Default|GetHasCollision) "QueryAndPhysics" "NoCollision")))

(fn ComponentstoSave
  (return 0))