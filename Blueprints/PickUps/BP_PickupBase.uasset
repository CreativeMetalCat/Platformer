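; Base pickup actor that the player collects by overlapping its box.
; On overlap with BP_Player it calls BePickedUp, which returns true here, and on success marks itself used, hides and plays a sound.
; If CanAutoRestock is set, a timer calls Restore after RestorationTime to show it and make it collectable again.
; The Used flag blocks repeat pickups, since hiding leaves collision untouched.
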(event OnComponentBeginOverlap(Box)
  (params (OverlappedComponent :type Primitive%20Component%20Object%20Reference) (OtherActor :type Actor%20Object%20Reference) (OtherComp :type Primitive%20Component%20Object%20Reference) (OtherBodyIndex :type Integer) (bFromSweep :type Boolean) (SweepResult :type Hit%20Result%20Structure%20%28by%20ref%29))
  (if (not (Variables|Default|GetUsed))
    (bind _asbp_player (Utilities|Casting|CastToBP_Player OtherActor))
    (bind _success (CallFunction|BePickedUp _asbp_player))
    (if _success
      (if (Variables|Default|GetCanAutoRestock)
        (bind _returnvalue (Utilities|Time|SetTimerbyFunctionName self "Restore" (Variables|Default|GetRestorationTime)))
        (Variables|Default|SetRestorationTimerHandle _returnvalue))
      (Variables|Default|SetUsed true)
      (Rendering|SetActorHiddenInGame true)
      (Audio|PlaySoundatLocation (Variables|Default|GetPickUpSound) (Transformation|GetActorLocation) "0, 0, 0" 1.0 1.0 0.0 0 0 0))))

(event EventBeginPlay)

(event Collision|EventActorBeginOverlap
  (params (OtherActor :type Actor%20Object%20Reference)))

(event EventTick
  (params (DeltaSeconds :type Float%20%28single-precision%29)))

(fn ConstructionScript)

(fn Restore
  (Variables|Default|SetUsed false)
  (Rendering|SetActorHiddenInGame false))

(fn BePickedUp
  (params (Human :type BP%20Human%20Base%20Object%20Reference))
  (return true))