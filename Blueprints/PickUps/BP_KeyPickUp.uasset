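; Key pickup actor that grants one key, identified by its KeyId, to the human who picks it up.
; Its BePickedUp override calls the parent, sends PickUpKey to the Human, plays a pickup sound at its location, destroys itself and returns true.
; The event graph holds only disabled default events, so all of its own logic lives in that override.
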(event EventBeginPlay
  (|CallParentFunction) ; This node is disabled and will not be called.\nDrag off pins to build functionality.
)

(event Collision|EventActorBeginOverlap
  (params (OtherActor :type Actor%20Object%20Reference))
  (|CallParentFunction OtherActor) ; This node is disabled and will not be called.\nDrag off pins to build functionality.
)

(event EventTick
  (params (DeltaSeconds :type Float%20%28single-precision%29))
  (|CallParentFunction DeltaSeconds) ; This node is disabled and will not be called.\nDrag off pins to build functionality.
)

(fn ConstructionScript
  (|CallParentFunction))

(fn BePickedUp
  (params (Human :type BP%20Human%20Base%20Object%20Reference))
  (|CallParentFunction 0)
  (Class|IPickups|PickUpKey(Message) Human (Variables|Default|GetKeyId) 1)
  (Audio|PlaySoundatLocation "/Game/Sounds/Interact/PickItem3.PickItem3" (Transformation|GetActorLocation) "0, 0, 0" 1.0 1.0 0.0 "/Game/SuperGrid/TutorialLevel/SoundEffects/Attenuation_Ambient.Attenuation_Ambient" 0 0)
  (Actor|DestroyActor)
  (return true))