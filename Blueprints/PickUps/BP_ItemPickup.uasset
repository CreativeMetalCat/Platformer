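; BP_ItemPickup is an item pickup actor that displays an item and slowly spins its meshes around the vertical axis on Tick.
; The construction script loads ItemInternal from the Item data table row, or uses its existing value when no table is set.
; It then applies either a skeletal or static mesh and hides the other component.
; BePickedUp passes ItemInternal to the Human's PickUpItemMessage and returns the result.
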(event EventBeginPlay
  (|CallParentFunction) ; This node is disabled and will not be called.\nDrag off pins to build functionality.
)

(event Collision|EventActorBeginOverlap
  (params (OtherActor :type Actor%20Object%20Reference))
  (|CallParentFunction OtherActor) ; This node is disabled and will not be called.\nDrag off pins to build functionality.
)

(event EventTick
  (params (DeltaSeconds :type Float%20%28single-precision%29))
  (|CallParentFunction DeltaSeconds)
  (Transformation|AddRelativeRotation (Variables|Default|GetSkeletalMesh) (Math|Rotator|MakeRotator 0.0 0.0 (* DeltaSeconds 2e+01)) false false))

(fn ConstructionScript
  (bind _item (Variables|Default|GetItem))
  (bind _skeletalmesh (Variables|Default|GetSkeletalMesh))
  (bind _staticmesh (Variables|Default|GetStaticMesh))
  (bind (_datatable _rowname) (Utilities|Struct|BreakDataTableRowHandle _item))
  (|CallParentFunction)
  (Utilities|IsValid _datatable
    (:Is%20Valid
      (bind _returnvalue (Utilities|GetDataTableRow _datatable _rowname)
        (:then
          (Variables|Default|SetItem_Internal _returnvalue))))
    (:Is%20Not%20Valid
      _))
  (if (.IsSkeletalMesh (Utilities|Struct|BreakS_CustomisationItem (Variables|Default|GetItem_Internal)))
    (Class|SkinnedMeshComponent|SetSkeletalMesh _skeletalmesh (.Mesh (Utilities|Struct|BreakS_CustomisationItem (Variables|Default|GetItem_Internal))) true)
    (Rendering|SetVisibility _staticmesh false false)
    (else
      (Components|StaticMesh|SetStaticMesh _staticmesh (.StaticMesh (Utilities|Struct|BreakS_CustomisationItem (Variables|Default|GetItem_Internal))))
      (Rendering|SetVisibility _skeletalmesh false false))))

(fn BePickedUp
  (params (Human :type BP%20Human%20Base%20Object%20Reference))
  (|CallParentFunction 0)
  (bind _success (Class|IPickups|PickUpItem(Message) Human (Variables|Default|GetItem_Internal)))
  (return _success))