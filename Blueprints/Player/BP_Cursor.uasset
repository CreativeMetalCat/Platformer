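; BP_Cursor is an actor that serves as an in-world mouse cursor positioned relative to the Player.
; Each tick, while the Player is not using a controller, it projects the Player to screen space and subtracts the mouse position.
; That pixel difference is applied directly as world units on Y and Z from the Player's location, with X held slightly offset.
; Debug prints are switched off, and deprojection nodes are left unused.
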(event EventBeginPlay)

(event Collision|EventActorBeginOverlap
  (params (OtherActor :type Actor%20Object%20Reference)))

(event EventTick
  (params (DeltaSeconds :type Float%20%28single-precision%29))
  (bind _player (Variables|Default|GetPlayer))
  (bind _returnvalue (Transformation|GetActorLocation _player))
  (bind (_x _y _z) (Math|Vector|BreakVector _returnvalue))
  (Utilities|IsValid _player
    (:Is%20Valid
      (bind _asplayer_controller (Utilities|Casting|CastToPlayerController (Pawn|GetController _player)))
      (if (not (Variables|/Game/Blueprints/Player/BP_Player.BP_Player_C|GetCurrentlyUsingController _player))
        (Transformation|SetActorLocation (Math|Vector|MakeVector (- _x 1e+01) (+ _y (- (.X (Math|Vector2D|BreakVector2D (.ScreenPosition (Class|GameplayStatics|ProjectWorldtoScreen _asplayer_controller _returnvalue false)))) (.LocationX (Game|Player|GetMousePosition _asplayer_controller)))) (+ _z (- (.Y (Math|Vector2D|BreakVector2D (.ScreenPosition (Class|GameplayStatics|ProjectWorldtoScreen _asplayer_controller _returnvalue false)))) (.LocationY (Game|Player|GetMousePosition _asplayer_controller))))) false false)
        (Development|PrintString (Utilities|String|Append "X: " (Utilities|String|ToString(Float) (.X (Math|Vector2D|BreakVector2D (.ScreenPosition (Class|GameplayStatics|ProjectWorldtoScreen _asplayer_controller _returnvalue false))))) " Y: " (Utilities|String|ToString(Float) (.Y (Math|Vector2D|BreakVector2D (.ScreenPosition (Class|GameplayStatics|ProjectWorldtoScreen _asplayer_controller _returnvalue false)))))) false false "(R=0.000000,G=0.660000,B=1.000000,A=1.000000)" DeltaSeconds)
        (Development|PrintString (Utilities|String|Append "X: " (Utilities|String|ToString(Float) (.X (Math|Vector2D|BreakVector2D (Math|Vector2D|MakeVector2D (.LocationX (Game|Player|GetMousePosition _asplayer_controller)) (.LocationY (Game|Player|GetMousePosition _asplayer_controller)))))) " Y: " (Utilities|String|ToString(Float) (.Y (Math|Vector2D|BreakVector2D (Math|Vector2D|MakeVector2D (.LocationX (Game|Player|GetMousePosition _asplayer_controller)) (.LocationY (Game|Player|GetMousePosition _asplayer_controller))))))) false false "(R=0.000000,G=1.000000,B=0.093123,A=1.000000)" DeltaSeconds)))))

(fn ConstructionScript)