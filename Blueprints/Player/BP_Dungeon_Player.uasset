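; Dungeon player Blueprint that adds key and item inventories, gated store access and ammo reloading to its parent class.
; Keys are counted per ID in a map and spent through UseKey, though PickUpKey looks up ID 0 for the existing count; items are unique.
; FinishReload refills the clip from the matching ammo reserve unless ammo is infinite.
; SetIsInRoom is empty, leaving its spring-arm zoom timeline unconnected.
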(event Custom|SetIsInRoom
  (params (Is :type Boolean)))

(event EventBeginPlay
  (|CallParentFunction) ; This node is disabled and will not be called.\nDrag off pins to build functionality.
)

(event Collision|EventActorBeginOverlap
  (params (OtherActor :type Actor%20Object%20Reference))
  (|CallParentFunction OtherActor) ; This node is disabled and will not be called.\nDrag off pins to build functionality.
)

(event EventTick
  (params (DeltaSeconds :type Float%20%28single-precision%29))
  (|CallParentFunction DeltaSeconds) ; This node is disabled and will not be called.\nDrag off pins to build functionality.
)

(event EventPickUpKey
  (params (Id :type Integer) (Amount :type Integer))
  (bind _keys (Variables|Default|GetKeys))
  (bind (_value _returnvalue) (Utilities|Map|Find _keys 0))
  (if _returnvalue
    (Utilities|Map|Add _keys Id (+ _value Amount))
    (else
      (Utilities|Map|Add _keys Id Amount))))

(fn ConstructionScript
  (|CallParentFunction))

(fn OpenStore
  (if (Variables|Default|GetCanUseStore)
    (|CallParentFunction)))

(fn HasKey
  (params (Id :type Integer))
  (bind _keys (Variables|Default|GetKeys))
  (bind (_value _returnvalue) (Utilities|Map|Find _keys Id))
  (if _returnvalue
    (return (> _value 0))
    (else
      (return false))))

(fn UseKey
  (params (Id :type Integer))
  (bind _keys (Variables|Default|GetKeys))
  (if (Keys|HasKey Id)
    (bind _output_get (LocalVariables|SetKeyAmount (.Value (Utilities|Map|Find _keys Id))))
    (Utilities|Map|Remove _keys Id)
    (if (> _output_get 1)
      (Utilities|Map|Add _keys Id (- _output_get 1)))))

(fn HasItem
  (params (Item :type S%20Customisation%20Item%20Structure))
  (return (!= (Utilities|Array|FindItem (Variables|Default|GetInventoryItems) Item) -1)))

(fn PickUpItem
  (params (Item :type S%20Customisation%20Item%20Structure))
  (if (not (CallFunction|HasItem Item))
    (Utilities|Array|Add (Variables|Default|GetInventoryItems) Item)
    (return true)
    (else
      (return false))))

(fn FinishReload
  (bind _ammo (Variables|Default|GetAmmo))
  (bind _weapon (Variables|Default|GetWeapon))
  (bind _ammotypeid (Variables|/Script/WeaponSystemPlugin.WeaponBase|GetAmmoTypeId _weapon))
  (bind _defaultammointheclip (Variables|/Script/WeaponSystemPlugin.WeaponBase|GetDefaultAmmoInTheClip _weapon))
  (Variables|Default|Setreloading false)
  (if (Variables|/Script/WeaponSystemPlugin.WeaponBase|GetbInfiniteAmmo _weapon)
    (Variables|/Script/WeaponSystemPlugin.WeaponBase|SetAmmoInTheClip _weapon (Variables|/Script/WeaponSystemPlugin.WeaponBase|GetDefaultAmmoInTheClip _weapon))
    (else
      (bind _keys (Utilities|Map|Keys _ammo))
      (if (!= (Utilities|Array|FindItem _keys _ammotypeid) -1)
        (bind _values (Utilities|Map|Values _ammo))
        (if (>= (Utilities|Array|Get(acopy) _values (Utilities|Array|FindItem _keys _ammotypeid)) (- _defaultammointheclip (Variables|/Script/WeaponSystemPlugin.WeaponBase|GetAmmoInTheClip _weapon)))
          (Utilities|Map|Add _ammo _ammotypeid (- (Utilities|Array|Get(acopy) _values (Utilities|Array|FindItem _keys _ammotypeid)) (- _defaultammointheclip (Variables|/Script/WeaponSystemPlugin.WeaponBase|GetAmmoInTheClip _weapon))))
          (Variables|/Script/WeaponSystemPlugin.WeaponBase|SetAmmoInTheClip _weapon _defaultammointheclip)
          (else
            (Variables|/Script/WeaponSystemPlugin.WeaponBase|SetAmmoInTheClip _weapon (+ (Variables|/Script/WeaponSystemPlugin.WeaponBase|GetAmmoInTheClip _weapon) (Utilities|Array|Get(acopy) _values (Utilities|Array|FindItem _keys _ammotypeid))))
            (Utilities|Map|Remove _ammo _ammotypeid)
            (Utilities|Map|Add _ammo _ammotypeid 0)))))))