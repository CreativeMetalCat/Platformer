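; BP_Camera is a player-controlled camera that brings up the main menu when flagged as the main-menu instance.
; On BeginPlay, if IsMainMenu is set, it creates UMG_MainMenu with IsInArena off and switches its player controller to UI-only input with a visible cursor.
; It also overlays UMG_IntroScreen when BP_PlatformerGameInstance reports the intro has not yet played.
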(event EventBeginPlay
  (if (Variables|Default|GetIsMainMenu)
    (bind _asplayer_controller (Utilities|Casting|CastToPlayerController (Pawn|GetController)))
    (bind _returnvalue (UserInterface|CreateWidget "/Game/Blueprints/UI/Menu/UMG_MainMenu.UMG_MainMenu_C" _asplayer_controller))
    (UserInterface|Viewport|AddtoViewport _returnvalue 0)
    (Input|SetInputModeUIOnly _asplayer_controller _returnvalue "DoNotLock")
    (Variables|/Script/Engine.PlayerController|SetbShowMouseCursor _asplayer_controller true)
    (bind _asbp_platformer_game_instance (Utilities|Casting|CastToBP_PlatformerGameInstance (Game|GetGameInstance)))
    (if (not (Variables|/Game/Blueprints/Player/BP_PlatformerGameInstance.BP_PlatformerGameInstance_C|GetIntroPlayed _asbp_platformer_game_instance))
      (bind _returnvalue_2 (UserInterface|CreateWidget "/Game/Blueprints/UI/intro/UMG_IntroScreen.UMG_IntroScreen_C"))
      (UserInterface|Viewport|AddtoViewport _returnvalue_2 0))))

(event Collision|EventActorBeginOverlap
  (params (OtherActor :type Actor%20Object%20Reference)))

(event EventTick
  (params (DeltaSeconds :type Float%20%28single-precision%29)))

(fn ConstructionScript)