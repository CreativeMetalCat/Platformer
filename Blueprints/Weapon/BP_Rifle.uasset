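; BP_Rifle is a rifle weapon that supplies its primary-fire effects and configures its collision for pickup.
; PrimaryFireEffects spawns the assault rifle muzzle flash at the weapon mesh's effects socket and plays the fire sound at the given location.
; The construction script enables capsule query and physics collision only when the rifle can be picked up, and always disables collision on the weapon mesh.
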(event EventBeginPlay)

(event Collision|EventActorBeginOverlap
  (params (OtherActor :type Actor%20Object%20Reference)))

(event EventTick
  (params (DeltaSeconds :type Float%20%28single-precision%29)))

(event EventPrimaryFireEffects
  (params (location :type Vector :default "0, 0, 0") (rotation :type Rotator :default "0, 0, 0"))
  (Effects|SpawnEmitteratLocation "/Game/models/MilitaryWeapDark/FX/P_AssaultRifle_MuzzleFlash.P_AssaultRifle_MuzzleFlash" (Transformation|GetSocketLocation (Variables|Default|GetWeaponMesh) (Utilities|String|StringToName (Variables|Default|GetWeaponEffectsSocketName))) rotation)
  (Audio|PlaySoundatLocation (Variables|Default|GetPrimaryFireSound) location "0, 0, 0" 1.0 1.0 0.0 0 0 0))

(fn ConstructionScript
  (bind _capsulecollisioncomponent (Variables|Default|GetCapsuleCollisionComponent))
  (if (Variables|Default|GetbCanBePickedUp)
    (Collision|SetCollisionEnabled _capsulecollisioncomponent "QueryAndPhysics")
    (else
      (Collision|SetCollisionEnabled _capsulecollisioncomponent "NoCollision")))
  (Collision|SetCollisionEnabled (Variables|Default|GetWeaponMesh) "NoCollision"))