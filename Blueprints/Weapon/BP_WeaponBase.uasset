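; BP_WeaponBase is the base weapon actor, which can act as a spinning world pickup.
; The CanBePickedUp flag enables capsule collision and mesh rotation on Tick, and the mesh itself never collides.
; A capsule overlap passes the weapon's class to BP_Player, and the weapon destroys itself if the player accepts it.
; PrimaryFireEffects spawns an assault rifle muzzle flash at the effects socket and plays the fire sound at a given location.
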(event OnComponentBeginOverlap(CapsuleCollisionComponent)
  (params (OverlappedComponent :type Primitive%20Component%20Object%20Reference) (OtherActor :type Actor%20Object%20Reference) (OtherComp :type Primitive%20Component%20Object%20Reference) (OtherBodyIndex :type Integer) (bFromSweep :type Boolean) (SweepResult :type Hit%20Result%20Structure%20%28by%20ref%29))
  (bind _asbp_player (Utilities|Casting|CastToBP_Player OtherActor))
  (bind _success (Class|IPickups|PickUpWeapon(Message) _asbp_player (Utilities|GetClass self)))
  (if _success
    (Actor|DestroyActor)))

(event EventBeginPlay
  (bind _capsulecollisioncomponent (Variables|Default|GetCapsuleCollisionComponent))
  (if (Variables|Default|GetbCanBePickedUp)
    (Collision|SetCollisionEnabled _capsulecollisioncomponent "QueryAndPhysics")
    (else
      (Collision|SetCollisionEnabled _capsulecollisioncomponent "NoCollision")))
  (Collision|SetCollisionEnabled (Variables|Default|GetWeaponMesh) "NoCollision"))

(event Collision|EventActorBeginOverlap
  (params (OtherActor :type Actor%20Object%20Reference)))

(event EventTick
  (params (DeltaSeconds :type Float%20%28single-precision%29))
  (if (Variables|Default|GetbCanBePickedUp)
    (Transformation|AddWorldRotation (Variables|Default|GetWeaponMesh) (Math|Rotator|MakeRotator 0.0 0.0 1.0) false false)))

(event EventPrimaryFireEffects
  (params (location :type Vector :default "0, 0, 0") (rotation :type Rotator :default "0, 0, 0"))
  (Effects|SpawnEmitteratLocation "/Game/models/MilitaryWeapDark/FX/P_AssaultRifle_MuzzleFlash.P_AssaultRifle_MuzzleFlash" (Transformation|GetSocketLocation (Variables|Default|GetWeaponMesh) (Utilities|String|StringToName (Variables|Default|GetWeaponEffectsSocketName))))
  (Audio|PlaySoundatLocation (Variables|Default|GetPrimaryFireSound) location "0, 0, 0" 1.0 1.0 0.0 0 0 0))

(fn ConstructionScript
  (bind _capsulecollisioncomponent (Variables|Default|GetCapsuleCollisionComponent))
  (if (Variables|Default|GetbCanBePickedUp)
    (Collision|SetCollisionEnabled _capsulecollisioncomponent "QueryAndPhysics")
    (else
      (Collision|SetCollisionEnabled _capsulecollisioncomponent "NoCollision")))
  (Collision|SetCollisionEnabled (Variables|Default|GetWeaponMesh) "NoCollision"))