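; BP_CameraArea is a trigger volume that moves the player's camera to a preset position when BP_Player enters it.
; On box overlap it caches the player and the camera actor's current location.
; A timeline then interpolates the camera from that location to the area's own position plus a Location offset.
; Nothing handles leaving the area, and only the camera's location changes, not its rotation.
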(event OnComponentBeginOverlap(Box)
  (params (OverlappedComponent :type Primitive%20Component%20Object%20Reference) (OtherActor :type Actor%20Object%20Reference) (OtherComp :type Primitive%20Component%20Object%20Reference) (OtherBodyIndex :type Integer) (bFromSweep :type Boolean) (SweepResult :type Hit%20Result%20Structure%20%28by%20ref%29))
  (bind _asbp_player (Utilities|Casting|CastToBP_Player OtherActor))
  (Variables|Default|SetTEMPPlayer _asbp_player)
  (bind _output_get (Variables|Default|SetOriginalLocation (Transformation|GetActorLocation (Variables|/Game/Blueprints/Player/BP_Player.BP_Player_C|GetCamera (Variables|Default|GetTEMPPlayer)))))
  (bind _cameramovement (Timeline|CameraMovementTimeline PlayFromStart)
    (:Update
      (Transformation|SetActorLocation (Variables|/Game/Blueprints/Player/BP_Player.BP_Player_C|GetCamera (Variables|Default|GetTEMPPlayer)) (+ _output_get (* (- (+ (Variables|Default|GetLocation) (Transformation|GetActorLocation)) _output_get) _cameramovement)) false false))))

(event EventBeginPlay)

(event Collision|EventActorBeginOverlap
  (params (OtherActor :type Actor%20Object%20Reference)))

(event EventTick
  (params (DeltaSeconds :type Float%20%28single-precision%29)))

(fn ConstructionScript)